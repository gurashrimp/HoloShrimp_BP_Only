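; Demo actor whose static mesh fades colour when something overlaps its box and turns into a sphere mesh when hit.
; BeginPlay creates a dynamic material instance from the mesh's first material and enables player input.
; Box begin overlap plays a timeline that drives the material's Colour parameter, and end overlap reverses it.
; A ChangingColor flag ignores overlap events while a fade is running.
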(event `self.ReceiveBeginPlay`
  (bind _staticmesh (`self.StaticMesh`))
  (bind _returnvalue (`PrimitiveComponent.CreateDynamicMaterialInstance` _staticmesh 0 (`PrimitiveComponent.GetMaterial` _staticmesh 0) "None"))
  (set `self.NewVar` _returnvalue)
  (`self.EnableInput` (`GameplayStatics.GetPlayerController` 0)))

(event `Key|F`
  (params (Key :type "Key Structure")))

(event `self.StaticMesh.OnComponentHit`
  (params (HitComponent :type "PrimitiveComponent Object Reference") (OtherActor :type "Actor Object Reference") (OtherComp :type "PrimitiveComponent Object Reference") (NormalImpulse :type "Vector Structure") (Hit :type "HitResult Structure (by ref)"))
  (`StaticMeshComponent.SetStaticMesh` (`self.StaticMesh`) "/Engine/EngineMeshes/Sphere.Sphere"))

(event `self.Box.OnComponentBeginOverlap`
  (params (OverlappedComponent :type "PrimitiveComponent Object Reference") (OtherActor :type "Actor Object Reference") (OtherComp :type "PrimitiveComponent Object Reference") (OtherBodyIndex :type Integer) (bFromSweep :type Boolean) (SweepResult :type "HitResult Structure (by ref)"))
  (if (not (`self.ChangingColor?`))
    (set `self.ChangingColor?` true)
    (bind (_direction _colour_fade) (`Timeline|Timeline` :!via `PlayFromStart` :!label _label)
      (:`Update`
        (`MaterialInstanceDynamic.SetVectorParameterValue` (`self.NewVar`) "Colour" _colour_fade))
      (:`Finished`
        (set `self.ChangingColor?` false)))))

(event `self.Box.OnComponentEndOverlap`
  (params (OverlappedComponent :type "PrimitiveComponent Object Reference") (OtherActor :type "Actor Object Reference") (OtherComp :type "PrimitiveComponent Object Reference") (OtherBodyIndex :type Integer))
  (if (not (`self.ChangingColor?`))
    (set `self.ChangingColor?` true)
    (goto _label :!via `Reverse`)))

(fn `UserConstructionScript`)